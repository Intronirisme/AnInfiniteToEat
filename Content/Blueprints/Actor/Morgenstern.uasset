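; Morgenstern is a moving weapon pawn that damages any Monster it overlaps, then calls its inherited Approach.
; It calls Approach on BeginPlay, and its Attack triples movement speed for an AI MoveTo.
; The destination is the normalized direction toward the player times ApproachDistance scaled by player life percentage, with no actor location added.
; Whether the move succeeds or fails, it waits for the attack-speed delay before approaching again.
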(event `self.ReceiveBeginPlay`
  (`parent.ReceiveBeginPlay`)
  (`self.Approach`))

(event `self.Attack`
  (bind (_props_life _props_attack _props_defense _props_attackspeed) (break `/Game/Blueprints/Misc/Stats` (`self.Props`)))
  (bind _daplayer (`self.daPlayer`))
  (set `FloatingPawnMovement.MaxSpeed` (* (`self.Speed`) 3.0) (`self.FloatingPawnMovement`))
  (`|AIMoveTo` null (* (`KismetMathLibrary.Normal` (- (`self.K2_GetActorLocation` _daplayer) (`self.K2_GetActorLocation`))) (* (/ (`/Game/Blueprints/Actor/Monster.LifePourcentage` _daplayer) 50.0) (`self.ApproachDistance`))) null 5.0 true
    (:`OnSuccess`
      _)
    (:`OnFail`
      _))
  (`KismetSystemLibrary.Delay` _props_attackspeed)
  (`self.Approach`))

(event `self.ReceiveActorBeginOverlap`
  (params (OtherActor :type "Actor Object Reference"))
  (bind (_props_life _props_attack) (break `/Game/Blueprints/Misc/Stats` (`self.Props`)))
  (bind _asmonster (cast `/Game/Blueprints/Actor/Monster` OtherActor))
  (`GameplayStatics.ApplyDamage` _asmonster _props_attack)
  (`self.Approach`))

(fn `UserConstructionScript`
  (`parent.UserConstructionScript`))