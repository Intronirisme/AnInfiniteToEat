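; Projectile actor that flies in a straight line and damages any Monster its Sphere overlaps.
; A Props vector packs sprite scale, speed and damage, with Tick offsetting the actor along Direction without sweep.
; The construction script scales the Canvas, feeds Sprite into a dynamic M_SpriteMaster material and yaws the actor to face Direction.
; Hits do not destroy the projectile in this graph.
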(event `self.ReceiveTick`
  (params (DeltaSeconds :type "Float (single-precision)"))
  (bind (_props_x _props_y) (`KismetMathLibrary.BreakVector` (`self.Props`)))
  (`self.K2_AddActorWorldOffset` (* (`self.Direction`) (* DeltaSeconds _props_y))))

(event `self.Sphere.OnComponentBeginOverlap`
  (params (OverlappedComponent :type "PrimitiveComponent Object Reference") (OtherActor :type "Actor Object Reference") (OtherComp :type "PrimitiveComponent Object Reference") (OtherBodyIndex :type Integer) (bFromSweep :type Boolean) (SweepResult :type "HitResult Structure (by ref)"))
  (bind (_props_x _props_y _props_z) (`KismetMathLibrary.BreakVector` (`self.Props`)))
  (cast `/Game/Blueprints/Actor/Monster` OtherActor)
  (`GameplayStatics.ApplyDamage` null _props_z))

(fn `UserConstructionScript`
  (bind (_direction_x _direction_y) (`KismetMathLibrary.BreakVector` (`self.Direction`)))
  (bind _props_x (`KismetMathLibrary.BreakVector` (`self.Props`)))
  (`SceneComponent.SetWorldScale3D` (`self.Canvas`) (`KismetMathLibrary.MakeVector` _props_x _props_x _props_x))
  (bind _returnvalue (`PrimitiveComponent.CreateDynamicMaterialInstance` (`self.Canvas`) 0 "/Game/Materials/M_SpriteMaster.M_SpriteMaster" "None"))
  (`MaterialInstanceDynamic.SetTextureParameterValue` _returnvalue "Sprite" (`self.sprite`))
  (`self.K2_SetActorRotation` (`KismetMathLibrary.MakeRotator` 0.0 0.0 (`KismetMathLibrary.DegAtan2` _direction_y _direction_x))))