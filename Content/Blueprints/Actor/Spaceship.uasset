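; Spaceship is an actor that takes damage, shows a health bar and can be eaten by the player.
; On BeginPlay it creates a HealthBar widget bound to itself and assigns it to its Health widget component.
; Each hit lowers Life and, while Life stays positive, shows the bar for a second through a retriggerable delay.
; Once Life runs out, a Player damage causer calls Eat with the ship's Stats.
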(event `self.ReceiveBeginPlay`
  (bind _returnvalue (`|CreateWidget` "/Game/HUD/HealthBar.HealthBar_C" null self))
  (`WidgetComponent.SetWidget` (`self.health`) _returnvalue))

(event `self.ReceiveAnyDamage`
  (params (Damage :type "Float (single-precision)") (DamageType :type "DamageType Object Reference") (InstigatedBy :type "Controller Object Reference") (DamageCauser :type "Actor Object Reference"))
  (bind _output_get (set `self.Life` (- (`self.Life`) Damage)))
  (if (> _output_get 0.0)
    ;[1 1 1] Show health bar for 1 sec on damage
    (`SceneComponent.SetVisibility` (`self.health`) true false)
    (`KismetSystemLibrary.RetriggerableDelay` 1.0)
    (`SceneComponent.SetVisibility` (`self.health`) false false)
    (else
      (bind _asplayer (cast `/Game/Blueprints/Actor/Player` DamageCauser))
      (`/Game/Blueprints/Actor/Player.Eat` _asplayer (`self.Stats`)))))

(fn `UserConstructionScript`)