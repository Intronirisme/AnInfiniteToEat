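; Player-controlled monster pawn that grows by eating, with Eat adding bonus life, attack, defence, attack speed and range.
; Tick scales the body by life percentage, derives a speed multiplier that rises as life drops, and applies it to axis movement input.
; Pivots turn the appendage along the travel direction and the mouth by mouse coordinates.
; Fire runs an attack timeline that only prints placeholder crunch messages.
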(event `self.ReceiveBeginPlay`
  ;[1 1 1] Init Creature
  (set `self.BaseScale` (`SceneComponent.RelativeScale3D` (`self.DefaultSceneRoot`))))

(event `self.ReceiveTick`
  (params (DeltaSeconds :type "Float (single-precision)"))
  (bind (_returnvalue_x _returnvalue_y) (`KismetMathLibrary.BreakVector` (`KismetMathLibrary.Vector_Normal2D` (- (`self.MousePosition`) (0.0 0.0 0.0)))))
  (bind (_returnvalue_x_2 _returnvalue_y_2) (`KismetMathLibrary.BreakVector` (`KismetMathLibrary.Normal` (- (`SceneComponent.K2_GetComponentLocation` (`self.DefaultSceneRoot`)) (`self.MonsterPosition`)))))
  ;[1 1 1] Change Scale On Life
  (`SceneComponent.SetWorldScale3D` (`self.DefaultSceneRoot`) (* (`self.BaseScale`) (`self.LifePourcentage`)))
  ;[1 1 1] Change Speed On Life
  (set `self.SpeedPourcentage` (+ 100.0 (- 100.0 (`self.LifePourcentage`))))
  ;[1 1 1] Set Appendice Position
  (`SceneComponent.K2_SetRelativeRotation` (`self.pivotAppendice`) (`KismetMathLibrary.MakeRotator` 0.0 0.0 (`KismetMathLibrary.DegAtan2` _returnvalue_y_2 _returnvalue_x_2)) false false)
  (set `self.MonsterPosition` (`SceneComponent.K2_GetComponentLocation` (`self.DefaultSceneRoot`)))
  ;[1 1 1] Set Mouth Position
  (`SceneComponent.K2_SetRelativeRotation` (`self.pivotmouth`) (`KismetMathLibrary.MakeRotator` 0.0 0.0 (`KismetMathLibrary.DegAtan2` _returnvalue_y _returnvalue_x)) false false)
  (set `self.MousePosition` (`KismetMathLibrary.MakeVector` (`self.MouseX`) (`self.MouseY`))))

(event `InputAction|Fire`
  (params (Key :type "Key Structure"))
  ;[1 1 1] Attack
  (:`Pressed`
    (set `self.InAttack?` true)
    (if (`self.InAttack?`)
      (`Timeline|Timeline_0` :!via `PlayFromStart` :!label _label
        (:`Update`
          (`KismetSystemLibrary.PrintString` "crounch crounch"))
        (:`Finished`
          (`KismetSystemLibrary.PrintString` "stopcrounch.")))))
  (:`Released`
    (set `self.InAttack?` false)
    (`KismetSystemLibrary.PrintString` "stopcrounch.")
    (goto _label :!via `Stop`)))

(event `InputAxis|Forward`
  (params (AxisValue :type "Float (single-precision)"))
  ;[1 1 1] Movement On Speed%
  (`self.AddMovementInput` (`SceneComponent.GetForwardVector` (`self.DefaultSceneRoot`)) (* AxisValue (/ (`self.SpeedPourcentage`) 100.0))))

(event `InputAxis|Right`
  (params (AxisValue :type "Float (single-precision)"))
  ;[1 1 1] Movement On Speed%
  (`self.AddMovementInput` (`SceneComponent.GetRightVector` (`self.DefaultSceneRoot`)) (* AxisValue (/ (`self.SpeedPourcentage`) 100.0))))

(fn `Eat`
  (params (bonusStats :type "/Game/Blueprints/Misc/Stats Structure"))
  ;[1 1 1] Add Life
  (set `self.LifePourcentage` (+ bonusStats_Life_6_2247E6B1499F7A6923A03B9D0337CABC (`self.LifePourcentage`)))
  ;[1 1 1] Add Attack
  (set `self.Attack` (+ bonusStats_Attack_15_6C13EA574A0B537337BA8BB047122414 (`self.Attack`)))
  ;[1 1 1] Add Defence
  (set `self.Defence` (+ bonusStats_Defense_8_DB63BE094F429EC95BEF06ADEE38E184 (`self.Defence`)))
  ;[1 1 1] Add AttackSpeed
  (set `self.AttackSpeed` (+ bonusStats_AttackSpeed_2_8392493347A28FA6BB8C75B20C1AFF99 (`self.AttackSpeed`)))
  ;[1 1 1] Add Range
  (set `self.MaxRange` (+ bonusStats_Range_12_8A146B1146F73353BB1464A1A0B04993 (`self.MaxRange`))))

(fn `UserConstructionScript`)