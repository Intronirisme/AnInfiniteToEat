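; Spawner actor that creates enemy SpaceshipV2 ships at its own transform while their level-wide count is below MaxMob.
; BeginPlay binds Spawn to a non-looping, zero-time timer, with no rescheduling in the graph.
; Spawn randomly picks one of two archetypes, using Select nodes to set sprite, speeds, pattern, stats and malus stats.
; The first archetype also randomizes its sprite, and the remaining Select options are unreachable.
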(event `self.ReceiveBeginPlay`
  (`KismetSystemLibrary.K2_SetTimerDelegate` (delegate `Spawn`)))

(event `Spawn`
  (bind _spawntype (`self.spawnType`))
  (bind _outactors (`GameplayStatics.GetAllActorsOfClass` "/Game/Blueprints/Actor/SpaceshipV2.SpaceshipV2_C"))
  (if (< (`KismetArrayLibrary.Array_Length` _outactors) (`self.maxMob`))
    (set `self.spawnType` (`KismetMathLibrary.RandomIntegerInRange` 0 1))
    (`|SpawnActorFromClass` "/Game/Blueprints/Actor/SpaceshipV2.SpaceshipV2_C" (`self.GetTransform`) "Undefined" "OverrideRootScale" null (select `int` _spawntype :`0` (select `bool` (`KismetMathLibrary.RandomBool`) :`false` "/Game/Sprites/Props/sputnik.sputnik" :`true` "/Game/Sprites/Props/estazioncosmico.estazioncosmico" :!type "Texture2D Object Reference") :`1` "/Game/Sprites/Spaceship/morgenstern1.morgenstern1" :`2` null :`3` null :`4` null) (select `int` _spawntype :`0` 200.0 :`1` 400.0 :`2` 0.0 :`3` 0.0 :`4` 0.0 :!type "Float (single-precision)") (select `int` _spawntype :`0` 200.0 :`1` 800.0 :`2` 0.0 :`3` 0.0 :`4` 0.0 :!type "Float (single-precision)") (select `int` _spawntype :`0` "NewEnumerator2" :`1` "NewEnumerator3" :`2` "NewEnumerator4" :`3` "NewEnumerator5" :`4` "NewEnumerator6" :!type "/Game/Blueprints/Misc/SpaceshipTypes Enum") (select `int` _spawntype :`0` (make `/Game/Blueprints/Misc/Stats` 1.0 0.0 3.0 1.0) :`1` (make `/Game/Blueprints/Misc/Stats` 2.0) :`2` (struct) :`3` (struct) :`4` (struct)) (select `int` _spawntype :`0` (struct) :`1` (make `/Game/Blueprints/Misc/Stats` 15.0 0.0 0.05) :`2` (struct) :`3` (struct) :`4` (struct)) null)))

(fn `UserConstructionScript`)