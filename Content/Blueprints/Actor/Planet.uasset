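; Planet actor that circles its origin and can be eaten by a Monster for a NutritiveScore reward.
; The construction script sets its sprite texture, scale and orbit offset, and Tick yaws the actor to move it around.
; A looping timer, unpaused only while a Monster overlaps the Sphere, shrinks the Canvas in steps.
; At minimum size, it calls Eat on that Monster and destroys itself.
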(event `self.ReceiveBeginPlay`
  (bind _returnvalue (`KismetSystemLibrary.K2_SetTimerDelegate` (delegate `Die`) 0.5 true))
  (bind _output_get (set `self.damageTimer` _returnvalue))
  (`KismetSystemLibrary.K2_PauseTimerHandle` _output_get))

(event `Die`
  (bind _canvas (`self.Canvas`))
  (bind _returnvalue_x (`KismetMathLibrary.BreakVector` (`SceneComponent.K2_GetComponentScale` _canvas)))
  (bind _returnvalue (- _returnvalue_x 0.1))
  ;[1 1 1] Eat planet
  (`KismetSystemLibrary.PrintString` "panik")
  (if (> _returnvalue 0.3)
    (`SceneComponent.SetWorldScale3D` _canvas (`KismetMathLibrary.MakeVector` _returnvalue _returnvalue _returnvalue))
    (else
      (`/Game/Blueprints/Actor/Monster.Eat` (`self.daMonster`) (make `/Game/Blueprints/Misc/Stats` (`self.NutritiveScore`)))
      (`self.K2_DestroyActor`))))

(event `self.ReceiveTick`
  (params (DeltaSeconds :type "Float (single-precision)"))
  (`self.K2_AddActorWorldRotation` (`KismetMathLibrary.MakeRotator` 0.0 0.0 (* DeltaSeconds (`self.Speed`)))))

(event `self.Sphere.OnComponentBeginOverlap`
  (params (OverlappedComponent :type "PrimitiveComponent Object Reference") (OtherActor :type "Actor Object Reference") (OtherComp :type "PrimitiveComponent Object Reference") (OtherBodyIndex :type Integer) (bFromSweep :type Boolean) (SweepResult :type "HitResult Structure (by ref)"))
  (bind _asmonster (cast `/Game/Blueprints/Actor/Monster` OtherActor))
  (set `self.daMonster` _asmonster)
  (`KismetSystemLibrary.K2_UnPauseTimerHandle` (`self.damageTimer`)))

(event `self.Sphere.OnComponentEndOverlap`
  (params (OverlappedComponent :type "PrimitiveComponent Object Reference") (OtherActor :type "Actor Object Reference") (OtherComp :type "PrimitiveComponent Object Reference") (OtherBodyIndex :type Integer))
  (cast `/Game/Blueprints/Actor/Monster` OtherActor)
  (`KismetSystemLibrary.K2_PauseTimerHandle` (`self.damageTimer`)))

(fn `UserConstructionScript`
  (bind _scale (`self.Scale`))
  (bind _returnvalue (`PrimitiveComponent.CreateDynamicMaterialInstance` (`self.Canvas`) 0 "/Game/Materials/M_SpriteMaster.M_SpriteMaster" "None"))
  (bind _output_get (set `self.mat` _returnvalue))
  (`MaterialInstanceDynamic.SetTextureParameterValue` _output_get "Sprite" (`self.Planet`))
  (`SceneComponent.K2_SetRelativeLocation` (`self.Canvas`) (`KismetMathLibrary.MakeVector` (`self.OrbitRadius`)) false false)
  (`SceneComponent.SetWorldScale3D` (`self.Canvas`) (`KismetMathLibrary.MakeVector` _scale _scale _scale)))