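; Spaceship AI actor that roams around or closes in on the player Monster, which eats it when its life runs out.
; AIMoveTo loops alternate Approach and Attack by Pattern: Neutral wanders, Defensif dashes along the player's direction, with approach distance scaled by the player's life.
; Damage briefly shows a health bar, and WorldLooper events offset the ship when the world wraps.
; A dynamic-material sprite rotates to face velocity; Shoot is an empty stub.
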(event `self.ReceiveAnyDamage`
  (params (Damage :type "Float (single-precision)") (DamageType :type "DamageType Object Reference") (InstigatedBy :type "Controller Object Reference") (DamageCauser :type "Actor Object Reference"))
  ;[1 0.1667 0.1667 1 26] Damage
  (bind _output_get (set `self.Life` (- (`self.Life`) Damage)))
  (if (> _output_get 0.0)
    ;;[1 1 1] Show health bar for 1 sec on damage
    (`SceneComponent.SetVisibility` (`self.health`) true false)
    (`KismetSystemLibrary.RetriggerableDelay` 1.0)
    (`SceneComponent.SetVisibility` (`self.health`) false false)
    (else
      (`/Game/Blueprints/Actor/Monster.Eat` (`self.daPlayer`) (`self.Stats`)))))

(event `self.ReceiveBeginPlay`
  (bind _props_life (break `/Game/Blueprints/Misc/Stats` (`self.Props`)))
  ;[0.3763 1 0.239] Create health bar
  (set `self.Life` _props_life)
  (bind _returnvalue (`|CreateWidget` "/Game/HUD/HealthBar.HealthBar_C" null self))
  (`WidgetComponent.SetWidget` (`self.health`) _returnvalue)
  ;[1 0.533 0.1939] Bind event teleport when player is out of bound
  (bind _outactors (`GameplayStatics.GetAllActorsOfClass` "/Game/Blueprints/Actor/WorldLooper.WorldLooper_C"))
  (bind _output (`|GetArrayItem` _outactors))
  (`/Engine/EditorBlueprintResources/StandardMacros.IsValid` _output
    (:`Is Valid`
      (add `/Game/Blueprints/Actor/WorldLooper.TPspaceships` _output (delegate `TeleportThemAll`))
      ;[0.859 0.2522 1] Get reference to monster
      (bind _asmonster (cast `/Game/Blueprints/Actor/Monster` (`GameplayStatics.GetPlayerPawn` 0)))
      (set `self.DaPlayer` _asmonster)
      ;[1 1 1] Neutral behavior, no approach
      (if (`|EnumInequality` (`self.Pattern`) "NewEnumerator2")
        (`self.Approach`)
        (else
          (`self.Attack`))))))

(event `TeleportThemAll`
  (params (Offset :type "Vector Structure"))
  ;[1 0.533 0.1939] Bind event teleport when player is out of bound
  (`self.K2_AddActorWorldOffset` Offset false true))

(event `Approach`
  ;[0 1 0.2585] Approach behavior
  (if (`|EnumEquality` (`self.State`) "NewEnumerator0")
    (set `CharacterMovementComponent.MaxWalkSpeed` (`self.Speed`) (`self.CharacterMovement`))
    (`|AIMoveTo` self (`self.K2_GetActorLocation` (`self.daPlayer`)) null (`self.getSafeApproachDistance`)
      (:`then`
        (`KismetSystemLibrary.Delay` 5.0 :!label _label)
        (`self.Approach`))
      (:`OnSuccess`
        (set `self.State` "NewEnumerator2")
        (`self.Attack`))
      (:`OnFail`
        (goto _label)))
    (else
      (`KismetSystemLibrary.PrintString` "Hello"))))

(event `self.ReceiveTick`
  (params (DeltaSeconds :type "Float (single-precision)"))
  ;[0.4638 0.7848 1] Just ticking
  (`self.AlignSprite`))

(event `Attack`
  (bind _returnvalue (`self.K2_GetActorLocation`))
  (bind (_props_life _props_attack _props_defense _props_attackcooldown) (break `/Game/Blueprints/Misc/Stats` (`self.Props`)))
  (bind (_props_life_2 _props_attack_2 _props_defense_2 _props_attackcooldown_2 _props_range) (break `/Game/Blueprints/Misc/Stats` (`self.Props`)))
  (bind (_props_life_3 _props_attack_3 _props_defense_3 _props_attackcooldown_3 _props_range_2) (break `/Game/Blueprints/Misc/Stats` (`self.Props`)))
  (set `CharacterMovementComponent.MaxWalkSpeed` (`self.AttackSpeed`) (`self.CharacterMovement`))
  (switch `/Game/Blueprints/Misc/SpaceshipTypes` (`self.Pattern`)
    (:`NewEnumerator2`
      ;[1 1 1] Neutral behavior, just moving around
      (`|AIMoveTo` self (`NavigationSystemV1.K2_GetRandomLocationInNavigableRadius` (`self.GetNavAgentLocation`) _props_range_2 null null) null
        (:`OnSuccess`
          _)
        (:`OnFail`
          _)))
    (:`NewEnumerator3`
      ;[0.07855 0.84 1] Deffensive behavior
      (`|AIMoveTo` self (+ (* (`KismetMathLibrary.Normal` (- (`self.K2_GetActorLocation` (`self.DaPlayer`)) _returnvalue)) (* 2.0 _props_range)) _returnvalue) null
        (:`OnSuccess`
          _)
        (:`OnFail`
          _))))
  ;[1 0.5431 0.8998] Choosing next move
  (`KismetSystemLibrary.Delay` _props_attackcooldown)
  (if (and (> (`KismetMathLibrary.Vector_Distance` (`self.K2_GetActorLocation` (`self.DaPlayer`)) (`self.K2_GetActorLocation`)) (`self.getSafeApproachDistance`)) (`|EnumInequality` (`self.Pattern`) "NewEnumerator2"))
    (set `self.State` "NewEnumerator0")
    (`self.Approach`)
    (else
      (`self.Attack`))))

(fn `AlignSprite`
  (bind (_returnvalue_x _returnvalue_y) (`KismetMathLibrary.BreakVector` (`self.GetVelocity`)))
  (if (`KismetMathLibrary.BooleanNAND` (`KismetMathLibrary.NearlyEqual_FloatFloat` _returnvalue_x) (`KismetMathLibrary.NearlyEqual_FloatFloat` _returnvalue_y))
    (`SceneComponent.K2_SetRelativeRotation` (`self.Canvas`) (`KismetMathLibrary.MakeRotator` 0.0 0.0 (`KismetMathLibrary.DegAtan2` _returnvalue_y _returnvalue_x)) false false)))

(fn `getSafeApproachDistance`
  (returns (Distance :type "Float (double-precision)"))
  (bind (_props_life _props_attack _props_defense _props_attackcooldown _props_range) (break `/Game/Blueprints/Misc/Stats` (`self.Props`)))
  (return (* _props_range (/ (`/Game/Blueprints/Actor/Monster.LifePourcentage` (`self.daPlayer`)) 100.0))))

(fn `Shoot`
  (params (dir :type "Vector Structure")))

(fn `UserConstructionScript`
  (bind _returnvalue (`PrimitiveComponent.CreateDynamicMaterialInstance` (`self.Canvas`) 0 "/Game/Materials/M_SpriteMaster.M_SpriteMaster" "None"))
  (bind _output_get (set `self.SpriteMat` _returnvalue))
  (`MaterialInstanceDynamic.SetTextureParameterValue` _output_get "Sprite" (`self.Sprite`)))