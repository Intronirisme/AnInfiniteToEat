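; WorldLooper is an actor that wraps any actor leaving its TheWorld box to the opposite side, looping the play area.
; The construction script sizes the box from WorldSize; on end overlap, Teleport compares the actor's world X and Y against SideDetectorRange.
; The resulting offset uses WorldSize.Y for both axes, leaves Z unchanged, and is printed, then applied as a teleport.
; The trailing Player cast filters nothing.
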(event `self.TheWorld.OnComponentEndOverlap`
  (params (OverlappedComponent :type "PrimitiveComponent Object Reference") (OtherActor :type "Actor Object Reference") (OtherComp :type "PrimitiveComponent Object Reference") (OtherBodyIndex :type Integer))
  (bind _output_get (set `self.tpOffset` (`self.Teleport` (`self.K2_GetActorLocation` OtherActor))))
  (`KismetSystemLibrary.PrintString` (`KismetStringLibrary.Conv_VectorToString` _output_get))
  (`self.K2_AddActorWorldOffset` OtherActor _output_get false true)
  (cast `/Game/Blueprints/Actor/Player` OtherActor))

(fn `Teleport`
  (params (BasePosition :type "Vector Structure"))
  (returns (Offset :type "Vector Structure"))
  (bind _sidedetectorrange (`self.sideDetectorRange`))
  (bind (_baseposition_x _baseposition_y) (`KismetMathLibrary.BreakVector` (`local.BasePosition`)))
  (bind (_worldsize_x _worldsize_y) (`KismetMathLibrary.BreakVector` (`self.worldSize`)))
  (bind _sidedetectorrange_2 (`self.sideDetectorRange`))
  (bind _baseposition_x_2 (`KismetMathLibrary.BreakVector` (`local.BasePosition`)))
  (bind (_worldsize_x_2 _worldsize_y_2) (`KismetMathLibrary.BreakVector` (`self.worldSize`)))
  (return (`KismetMathLibrary.MakeVector` (`KismetMathLibrary.SelectFloat` _worldsize_y (`KismetMathLibrary.SelectFloat` (* -1 _worldsize_y) 0.0 (> _baseposition_x_2 _sidedetectorrange_2)) (< _baseposition_x_2 (* -1 _sidedetectorrange_2))) (`KismetMathLibrary.SelectFloat` _worldsize_y_2 (`KismetMathLibrary.SelectFloat` (* -1 _worldsize_y_2) 0.0 (> _baseposition_y _sidedetectorrange)) (< _baseposition_y (* -1 _sidedetectorrange))))))

(fn `UserConstructionScript`
  (`BoxComponent.SetBoxExtent` (`self.TheWorld`) (/ (`self.worldSize`) 2) false))